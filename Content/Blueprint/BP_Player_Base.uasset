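; Base player pawn that collects cow targets and gives audio feedback on its flight movement.
; Each tick, horizontal speed, vertical speed and rotation drive the pitch of three looping sounds, each muted below its threshold.
; On overlap it destroys the other actor, picks a random location, lifts it above any surface found by an upward trace, then spawns a new BP_Target with a pickup sound.
; Ring-modulation effect nodes are left unconnected.
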(event `self.ReceiveTick`
  (params (DeltaSeconds :type "Float (single-precision)"))
  (bind _returnvalue (`KismetMathLibrary.Abs` (`self.RotationValue`)))
  (bind (_velocity_x _velocity_y) (`KismetMathLibrary.BreakVector` (`MovementComponent.Velocity` (`self.FloatingPawnMovement`))))
  (bind (_velocity_x_2 _velocity_y_2 _velocity_z) (`KismetMathLibrary.BreakVector` (`MovementComponent.Velocity` (`self.FloatingPawnMovement`))))
  (bind _returnvalue_2 (`KismetMathLibrary.Abs` _velocity_z))
  (bind _returnvalue_3 (`KismetMathLibrary.Sqrt` (+ (`KismetMathLibrary.MultiplyMultiply_FloatFloat` _velocity_x 2.0) (`KismetMathLibrary.MultiplyMultiply_FloatFloat` _velocity_y 2.0))))
  (`|ExecutionSequence`
    (:`then_0`
      ;[1 1 1] Pitch Speed Sound
      (`AudioComponent.SetPitchMultiplier` (`self.SpeedSound`) (+ (* _returnvalue_3 (`self.SpeedPitchMultiplier`)) (`self.SpeedMinPitch`)))
      (`self.Mute Sound` (`self.SpeedSound`) _returnvalue_3 (`self.SpeedMinVelocity`)))
    (:`then_1`
      ;[1 1 1] Pitch Altitude Sound
      (`AudioComponent.SetPitchMultiplier` (`self.AltitudeSound`) (+ (* _returnvalue_2 (`self.AltitduePitchMultiplier`)) (`self.AltitudeMinPitch`)))
      (`self.Mute Sound` (`self.AltitudeSound`) _returnvalue_2 (`self.AltitudeMinVelocity`)))
    (:`then_2`
      ;[1 1 1] Rotation Pitch
      (`AudioComponent.SetPitchMultiplier` (`self.RotationSound`) (+ (* _returnvalue (`self.RotationPitchMultiplier`)) (`self.RotationMinPitch`)))
      (`self.Mute Sound` (`self.RotationSound`) _returnvalue (`self.RotationMinVelocity`)))))

(event `self.ReceiveActorBeginOverlap`
  (params (OtherActor :type "Actor Object Reference"))
  ;[1 1 1] Destroy the current cow and create a new one
  (`self.K2_DestroyActor` OtherActor)
  (`|ExecutionSequence`
    (:`then_0`
      (bind _output_get (`self.GenerateSpawnLocation`))
      (bind (_outhit _returnvalue) (`KismetSystemLibrary.LineTraceSingle` _output_get (+ _output_get (0.0 0.0 500.0)) "TraceTypeQuery1"))
      (if _returnvalue
        (set `self.spawnLocation` (+ (`.Location` (`GameplayStatics.BreakHitResult` _outhit)) (0.0 0.0 100.0)))))
    (:`then_1`
      (`self.SpawnCow` (`self.spawnLocation`)))))

(fn `GenerateSpawnLocation`
  (returns (Output_Get :type "Vector Structure"))
  (bind _output_get (set `self.spawnLocation` (`KismetMathLibrary.MakeVector` (`KismetMathLibrary.RandomFloatInRange` -5000.0 5000.0) (`KismetMathLibrary.RandomFloatInRange` -5000.0 5000.0) (`KismetMathLibrary.RandomFloatInRange` -50.0 500.0))))
  (return _output_get))

(fn `Mute Sound`
  (params (`Audio Component` :type "AudioComponent Object Reference") (`Current Velocity` :type "Float (double-precision)") (`Minimum Velocity` :type "Float (double-precision)"))
  (if (< `Current Velocity` `Minimum Velocity`)
    (`AudioComponent.SetVolumeMultiplier` `Audio Component` 0.0)
    (else
      (`AudioComponent.SetVolumeMultiplier` `Audio Component` 1.0))))

(fn `SpawnCow`
  (params (SpawnLocation :type "Vector Structure"))
  (`|SpawnActorFromClass` "/Game/Blueprint/BP_Target.BP_Target_C" (`KismetMathLibrary.MakeTransform` SpawnLocation) "AdjustIfPossibleButAlwaysSpawn" "OverrideRootScale" null null)
  (`AudioComponent.Play` (`self.PickUpSound`) 0.0))

(fn `UserConstructionScript`)