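; Player controller that turns axis input into movement for the possessed BP_Player pawn.
; MoveFwd and MoveUp add movement input along the pawn's forward and up vectors.
; MoveRight adds controller yaw input, so it turns the pawn instead of strafing.
; Each handler acts only when the controlled pawn is valid and casts to BP_Player.
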(event `InputAxis|MoveFwd`
  (params (AxisValue :type "Float (single-precision)"))
  (bind _returnvalue (`self.K2_GetPawn`))
  ;[1 1 1] Basic Input: Up/Down, Left/Right, Fwd/Bwd
  (`/Engine/EditorBlueprintResources/StandardMacros.IsValid` _returnvalue
    (:`Is Valid`
      (bind _asbp_player (cast `/Game/Blueprint/BP_Player` _returnvalue))
      (`Pawn.AddMovementInput` _asbp_player (`self.GetActorForwardVector` _returnvalue) AxisValue false))))

(event `InputAxis|MoveRight`
  (params (AxisValue :type "Float (single-precision)"))
  (bind _returnvalue (`self.K2_GetPawn`))
  ;[1 1 1] Basic Input: Up/Down, Left/Right, Fwd/Bwd
  (`/Engine/EditorBlueprintResources/StandardMacros.IsValid` _returnvalue
    (:`Is Valid`
      (cast `/Game/Blueprint/BP_Player` _returnvalue)
      (`Pawn.AddControllerYawInput` _returnvalue AxisValue))))

(event `InputAxis|MoveUp`
  (params (AxisValue :type "Float (single-precision)"))
  (bind _returnvalue (`self.K2_GetPawn`))
  ;[1 1 1] Basic Input: Up/Down, Left/Right, Fwd/Bwd
  (`/Engine/EditorBlueprintResources/StandardMacros.IsValid` _returnvalue
    (:`Is Valid`
      (bind _asbp_player (cast `/Game/Blueprint/BP_Player` _returnvalue))
      (`Pawn.AddMovementInput` _asbp_player (`self.GetActorUpVector` _returnvalue) AxisValue false))))

(fn `UserConstructionScript`)